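; BP_Cube is an overlap-triggered test actor for timing a print loop, labeled with its LoopCount on BeginPlay.
; On overlap it stores the real-time partial seconds and opens a trace region named from LoopCount.
; The loop has fixed 0..0 bounds, independent of LoopCount, and its body prints the index, closes the trace region and prints start minus current partial seconds.
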(event `self.ReceiveBeginPlay`
  ;[1 1 1] set the text to the loop count
  (`TextRenderComponent.K2_SetText` (`self.LoopCounter`) (`KismetTextLibrary.Conv_IntToText` (`self.LoopCount`))))

(event `self.ReceiveActorBeginOverlap`
  (params (OtherActor :type "Actor Object Reference"))
  (bind _returnvalue (`KismetStringLibrary.Concat_StrStr` (`KismetStringLibrary.Conv_IntToString` (`self.LoopCount`)) "BP_Cube"))
  ;[1 1 1] start recording time
  (set `self.Start` (`.PartialSeconds` (`GameplayStatics.GetAccurateRealTime`)))
  (`TraceUtilLibrary.TraceMarkRegionStart` _returnvalue)
  ;[1 1 1] loop Body
  (for _index (range 1)
    (`KismetSystemLibrary.PrintText` (`KismetTextLibrary.Conv_IntToText` _index))
    ;[1 1 1] End the trace and time
    (`TraceUtilLibrary.TraceMarkRegionEnd` _returnvalue)
    (`KismetSystemLibrary.PrintText` (`KismetTextLibrary.Conv_DoubleToText` (- (`self.Start`) (`.PartialSeconds` (`GameplayStatics.GetAccurateRealTime`))) "HalfToEven"))))

(fn `UserConstructionScript`)